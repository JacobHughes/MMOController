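; Player controller giving MMO-style mouse and keyboard control of an MMOCharacter and its boom camera.
; Left drag orbits the camera, right drag also steers control yaw, and the wheel zooms within limits.
; Movement follows yaw-only control rotation, slowed when backing up; the rotate axis turns, or strafes while a mouse button is held.
; Holding either button hides the cursor for game-only input; releasing both restores UI interaction.
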(event Input|ActionEvents|InputActionMouseScrollDown
  ;[1 1 1] Mouse wheel zoom
  (:Pressed
    (bind _asmmocharacter (Utilities|Casting|CastToMMOCharacter (Game|Player|GetPlayerPawn 0)))
    (Variables|/Script/Engine.SpringArmComponent|SetTargetArmLength (Variables|/Game/Blueprints/MMOCharacter.MMOCharacter_C|GetCameraBoom _asmmocharacter) (Math|Float|Clamp(Float) (+ (* (Variables|Default|GetZoomAmount) (Variables|Default|GetZoomSensitivity)) (Variables|/Script/Engine.SpringArmComponent|GetTargetArmLength (Variables|/Game/Blueprints/MMOCharacter.MMOCharacter_C|GetCameraBoom _asmmocharacter))) (Variables|Default|GetMinBoomLength) (Variables|Default|GetMaxBoomLength)))))

(event Input|ActionEvents|InputActionMouseScrollUp
  ;[1 1 1] Mouse wheel zoom
  (:Released
    (bind _asmmocharacter (Utilities|Casting|CastToMMOCharacter (Game|Player|GetPlayerPawn 0)))
    (Variables|/Script/Engine.SpringArmComponent|SetTargetArmLength (Variables|/Game/Blueprints/MMOCharacter.MMOCharacter_C|GetCameraBoom _asmmocharacter) (Math|Float|Clamp(Float) (- (Variables|/Script/Engine.SpringArmComponent|GetTargetArmLength (Variables|/Game/Blueprints/MMOCharacter.MMOCharacter_C|GetCameraBoom _asmmocharacter)) (* (Variables|Default|GetZoomAmount) (Variables|Default|GetZoomSensitivity))) (Variables|Default|GetMinBoomLength) (Variables|Default|GetMaxBoomLength)))))

(event Input|ActionEvents|InputActionLeftClick
  ;[1 1 1] Left Click changes interface interaction
  (:Pressed
    (Variables|Default|SetLeftMousePressed true)
    (CallFunction|ToggleUIControlOff))
  (:Released
    (Variables|Default|SetLeftMousePressed false)
    (if (not (Variables|Default|GetRightMousePressed))
      (CallFunction|ToggleUIControlon)
      (CallFunction|RotateCharactertoCamera))))

(event Input|ActionEvents|InputActionRightClick
  ;[1 1 1] Right click changes interface interaction
  (:Pressed
    (Variables|Default|SetRightMousePressed true)
    (CallFunction|ToggleUIControlOff))
  (:Released
    (Variables|Default|SetRightMousePressed false)
    (if (not (Variables|Default|GetLeftMousePressed))
      (CallFunction|ToggleUIControlon))))

(event Input|AxisEvents|InputAxisStrafeRight
  (params (AxisValue :type Float%20%28single-precision%29))
  ;[1 1 1] Forward and Right input axis control
  (CallFunction|AddStrafeInput AxisValue (Class|KismetMathLibrary|MakeRot 0.0 (.Yaw (Class|KismetMathLibrary|BreakRot (Pawn|GetControlRotation :!class /Script/Engine.Controller))) 0.0)))

(event Input|AxisEvents|InputAxisRotate
  (params (AxisValue :type Float%20%28single-precision%29))
  ;[1 1 1] Rotate axis control (rotate the character)
  (if (or (Variables|Default|GetRightMousePressed) (Variables|Default|GetLeftMousePressed))
    ;[1 1 1] If right mouse is pressed, we strafe not rotate
    (CallFunction|AddStrafeInput AxisValue (Class|KismetMathLibrary|MakeRot 0.0 (.Yaw (Class|KismetMathLibrary|BreakRot (Pawn|GetControlRotation :!class /Script/Engine.Controller))) 0.0))
    (else
      ;[1 1 1] No modifier control, turn on the spot
      (CallFunction|RotateCameraTurn AxisValue)
      (CallFunction|RotateCharactertoCamera)
      (Transformation|AddActorLocalRotation (Pawn|GetControlledPawn) (Class|KismetMathLibrary|MakeRot 0.0 (* AxisValue (Variables|Default|GetInputYawScale)) 0.0) false))))

(event Input|AxisEvents|InputAxisLookUp
  (params (AxisValue :type Float%20%28single-precision%29))
  ;[1 1 1] Left mouse drag rotates the camera
  (if (Variables|Default|GetLeftMousePressed)
    (CallFunction|RotateCameraLookUp AxisValue)))

(event Input|AxisEvents|InputAxisTurn
  (params (AxisValue :type Float%20%28single-precision%29))
  ;[1 1 1] Right Mouse Drag rotates Character and Camera
  (if (Variables|Default|GetRightMousePressed)
    (CallFunction|RotateCameraTurn AxisValue)
    (CallFunction|RotateCharactertoCamera)))

(event Input|AxisEvents|InputAxisLookUp
  (params (AxisValue :type Float%20%28single-precision%29))
  ;[1 1 1] Right Mouse Drag rotates Character and Camera
  (if (Variables|Default|GetRightMousePressed)
    (Class|PlayerController|AddPitchInput AxisValue)
    (CallFunction|RotateCameraLookUp AxisValue)))

(event Input|AxisEvents|InputAxisMoveForward
  (params (AxisValue :type Float%20%28single-precision%29))
  ;[1 1 1] Forward and Right input axis control
  (CallFunction|AddForwardInput AxisValue (Class|KismetMathLibrary|MakeRot 0.0 (.Yaw (Class|KismetMathLibrary|BreakRot (Pawn|GetControlRotation :!class /Script/Engine.Controller))) 0.0)))

(event Input|AxisEvents|InputAxisTurn
  (params (AxisValue :type Float%20%28single-precision%29))
  ;[1 1 1] Left mouse drag rotates the camera
  (if (Variables|Default|GetLeftMousePressed)
    (CallFunction|RotateCameraTurn AxisValue)))

(fn ConstructionScript)

(fn NewFunction0
  (params (PlayerPawn :type Pawn%20Object%20Reference) (Direction :type Vector) (AxisValue :type Float%20%28single-precision%29))
  (if (Variables|Default|GetMovingBackwards)
    (Pawn|Input|AddMovementInput PlayerPawn Direction (* AxisValue (Variables|Default|GetBackwardsSpeed)) false)
    (else
      (Pawn|Input|AddMovementInput PlayerPawn Direction AxisValue false)))
  (return))

(fn AddStrafeInput
  (params (AxisValue :type Float%20%28single-precision%29) (Rotation :type Rotator))
  (bind _returnvalue (Game|Player|GetPlayerPawn 0))
  (bind _returnvalue_2 (Math|Vector|GetRightVector Rotation))
  ;[1 1 1] Add strafing axis input. Scale if differently if moving backwards
  (if (Variables|Default|GetMovingBackwards)
    (Pawn|Input|AddMovementInput _returnvalue _returnvalue_2 (* AxisValue (Variables|Default|GetBackwardsSpeed)) false)
    (else
      (Pawn|Input|AddMovementInput _returnvalue _returnvalue_2 AxisValue false))))

(fn AddForwardInput
  (params (AxisValue :type Float%20%28single-precision%29) (Rotation :type Rotator))
  (bind _returnvalue (Game|Player|GetPlayerPawn 0))
  (bind _returnvalue_2 (Math|Vector|GetForwardVector Rotation))
  ;[1 1 1] Add forward axis input. If moving backwards, scale differently
  (Variables|Default|SetMovingBackwards (> 0.0 AxisValue))
  (if (Variables|Default|GetMovingBackwards)
    (Pawn|Input|AddMovementInput _returnvalue _returnvalue_2 (* AxisValue (Variables|Default|GetBackwardsSpeed)) false)
    (else
      (Pawn|Input|AddMovementInput _returnvalue _returnvalue_2 AxisValue false))))

(fn ToggleUIControlOff
  ;[1 1 1] Turn off the mouse cursor, interacting with UI, and locking the cursor to the game window
  (Input|SetInputModeGameOnly (Game|GetPlayerController 0))
  (Variables|Default|SetbShowMouseCursor false)
  (Variables|Default|SetbEnableClickEvents false)
  (Variables|Default|SetbEnableMouseOverEvents false))

(fn ToggleUIControlon
  ;[1 1 1] Turn on the mouse cursor, lock the mouse inside the game window, and allow interaction with UI
  (Input|SetInputModeGameandUI (Game|GetPlayerController 0) 0 true false)
  (Variables|Default|SetbShowMouseCursor true)
  (Variables|Default|SetbEnableClickEvents true)
  (Variables|Default|SetbEnableMouseOverEvents true))

(fn RotateCameraTurn
  (params (AxisValue :type Float%20%28single-precision%29))
  ;[1 1 1] Rotate the camera with the turn axis input (yaw)
  (bind _asmmocharacter (Utilities|Casting|CastToMMOCharacter (Game|Player|GetPlayerPawn 0)))
  (Transformation|SetWorldRotation (Variables|/Game/Blueprints/MMOCharacter.MMOCharacter_C|GetCameraBoom _asmmocharacter) (Class|KismetMathLibrary|MakeRot (.Pitch (Class|KismetMathLibrary|BreakRot (Transformation|GetWorldRotation (Variables|/Game/Blueprints/MMOCharacter.MMOCharacter_C|GetCameraBoom _asmmocharacter)))) (+ (* AxisValue (Variables|Default|GetInputYawScale)) (.Yaw (Class|KismetMathLibrary|BreakRot (Transformation|GetWorldRotation (Variables|/Game/Blueprints/MMOCharacter.MMOCharacter_C|GetCameraBoom _asmmocharacter))))) 0.0) false))

(fn RotateCameraLookUp
  (params (AxisValue :type Float%20%28single-precision%29))
  (bind _playercameramanager (Variables|Default|GetPlayerCameraManager))
  ;[1 1 1] Rotate the camera with the LookUp axis input (pitch)
  (bind _asmmocharacter (Utilities|Casting|CastToMMOCharacter (Game|Player|GetPlayerPawn 0)))
  (Transformation|SetWorldRotation (Variables|/Game/Blueprints/MMOCharacter.MMOCharacter_C|GetCameraBoom _asmmocharacter) (Class|KismetMathLibrary|MakeRot (Math|Float|Clamp(Float) (+ (* AxisValue (Variables|Default|GetInputPitchScale)) (.Pitch (Class|KismetMathLibrary|BreakRot (Transformation|GetWorldRotation (Variables|/Game/Blueprints/MMOCharacter.MMOCharacter_C|GetCameraBoom _asmmocharacter))))) (Variables|/Script/Engine.PlayerCameraManager|GetViewPitchMin _playercameramanager) (Variables|/Script/Engine.PlayerCameraManager|GetViewPitchMax _playercameramanager)) (.Yaw (Class|KismetMathLibrary|BreakRot (Transformation|GetWorldRotation (Variables|/Game/Blueprints/MMOCharacter.MMOCharacter_C|GetCameraBoom _asmmocharacter)))) 0.0) false))

(fn RotateCharactertoCamera
  ;[1 1 1] Update the player controller rotation to the camera orientation
  (bind _asmmocharacter (Utilities|Casting|CastToMMOCharacter (Game|Player|GetPlayerPawn 0)))
  (Pawn|SetControlRotation (Class|KismetMathLibrary|MakeRot 0.0 (.Yaw (Class|KismetMathLibrary|BreakRot (Variables|/Script/Engine.SceneComponent|GetRelativeRotation (Variables|/Game/Blueprints/MMOCharacter.MMOCharacter_C|GetCameraBoom _asmmocharacter)))) 0.0)))